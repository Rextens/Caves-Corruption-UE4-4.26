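; Player character Blueprint that handles toolbar selection, equipment and quit UIs, 3D item crafting and save/load.
; Crafting hides the world and spawns a CraftingProcess, where clicks attach or remove item meshes at the nearest unlocked sockets.
; Closing with C recursively flattens that component tree into a JSON-derived string, matched against one hardcoded test recipe.
; SaveGame slots per world name store player, world and placed items; only player loading is implemented.
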(event EventBeginPlay
  (bind _returnvalue (Game|GetPlayerController 0))
  (bind _returnvalue_2 (UserInterface|CreateWidget "/Game/Components/UI/ToolBar_BP.ToolBar_BP_C" _returnvalue))
  (bind _output_get (Variables|Default|SetToolBar _returnvalue_2))
  (UserInterface|Viewport|AddtoViewport _output_get 0)
  (bind _returnvalue_3 (SaveGame|CreateSaveGameObject "/Game/SaveStructs/savePlayer.savePlayer_C"))
  (Variables|Default|SetsaveInstance _returnvalue_3)
  (bind _returnvalue_4 (UserInterface|CreateWidget "/Game/Components/UI/ItemStatsShow.ItemStatsShow_C" _returnvalue))
  (Variables|Default|SetItemStatsShow _returnvalue_4))

(event Collision|EventActorBeginOverlap
  (params (OtherActor :type Actor%20Object%20Reference)))

(event EventTick
  (params (DeltaSeconds :type Float%20%28single-precision%29))
  (if (not (not (Variables|Default|GetisCraftingOpened)))
    (Transformation|AddWorldRotation (Variables|/Script/Engine.Actor|GetRootComponent (Variables|Default|GetcraftingProcess)) (Math|Rotator|MakeRotator (Class|Actor|GetInputAxisKeyValue) 0.0 (Class|Actor|GetInputAxisKeyValue)) false false)))

(event Input|KeyboardEvents|E
  (params (Key :type Key%20Structure :default "None"))
  (bind _returnvalue (Game|GetPlayerController 0))
  (:Pressed
    (if (not (Variables|Default|GetEscapeMenu))
      (if (and (not (Variables|Default|GetisCraftingOpened)) (not (Variables|Default|GetisGuiOpen)))
        (bind _returnvalue_2 (UserInterface|CreateWidget "/Game/Components/UI/Equipment_BP.Equipment_BP_C" _returnvalue))
        (bind _output_get (Variables|Default|Setequipment _returnvalue_2))
        (UserInterface|Viewport|AddtoViewport _output_get 0)
        (Utilities|Array|Add (Variables|Default|GetcurrentlyOpenUIs) _output_get)
        (bind _returnvalue_3 (UserInterface|CreateWidget "/Game/Components/UI/ItemStatsShow.ItemStatsShow_C" _returnvalue))
        (Variables|Default|SetItemStatsShow _returnvalue_3)
        (Widget|RemovefromParent (Variables|Default|GetToolBar))
        (Variables|/Script/Engine.PlayerController|SetbShowMouseCursor _returnvalue true)
        (Variables|Default|SetisGuiOpen true)
        (Input|SetInputModeGameandUI _returnvalue (Variables|Default|Getequipment) "LockAlways" true)
        (Variables|Default|SetshowItemStats true)
        (else
          (CallFunction|CloseGuis)
          (UserInterface|Viewport|AddtoViewport (Variables|Default|GetToolBar) 0))))))

(event Input|KeyboardEvents|F1
  (params (Key :type Key%20Structure :default "None"))
  (:Pressed
    (Utilities|FlowControl|FlipFlop
      (:A
        (Widget|RemovefromParent (Variables|Default|GetToolBar)))
      (:B
        (UserInterface|Viewport|AddtoViewport (Variables|Default|GetToolBar) 0)))))

(event Input|MouseEvents|LeftMouseButton
  (params (Key :type Key%20Structure :default "None"))
  (:Pressed
    (if (Variables|Default|GetisCraftingOpened)
      (if (== (Variables|/Script/Engine.StaticMeshComponent|GetStaticMesh (Variables|/Game/Components/crafting/craftingProcess.craftingProcess_C|Getmesh (Variables|Default|GetcraftingProcess))) 0)
        (CallFunction|EmptyProcess)
        (else
          (CallFunction|AddChildCraftingItem))))))

(event Input|MouseEvents|RightMouseButton
  (params (Key :type Key%20Structure :default "None"))
  (:Pressed
    (if (Variables|Default|GetisCraftingOpened)
      (CallFunction|RemoveItemfromCraftingProcess))))

(event Input|MouseEvents|MouseWheelUp
  (params (Key :type Key%20Structure :default "None"))
  (:Pressed
    (Default|BringBackUnselectedItemFrame (Variables|Default|GetToolBar))
    (bind _output_get (Variables|Default|SetselectedItem (+ (Variables|Default|GetselectedItem) 1)))
    (if (> _output_get 8)
      (Variables|Default|SetselectedItem 0))
    (Default|ChangeSelectedItemPosition (Variables|Default|GetToolBar))
    (Class|PlayerCharacter|ChangeItemMeshinHand)))

(event Input|MouseEvents|MouseWheelDown
  (params (Key :type Key%20Structure :default "None"))
  (:Pressed
    (Default|BringBackUnselectedItemFrame (Variables|Default|GetToolBar))
    (bind _output_get (Variables|Default|SetselectedItem (- (Variables|Default|GetselectedItem) 1)))
    (if (< _output_get 0)
      (Variables|Default|SetselectedItem 8))
    (Default|ChangeSelectedItemPosition (Variables|Default|GetToolBar))
    (Class|PlayerCharacter|ChangeItemMeshinHand)))

(event Input|KeyboardEvents|P
  (params (Key :type Key%20Structure :default "None"))
  (bind _returnvalue (Game|GetPlayerController 0))
  (:Pressed
    (if (not (Variables|Default|GetEscapeMenu))
      (bind _returnvalue_2 (UserInterface|CreateWidget "/Game/Components/UI/QuitMenu.QuitMenu_C"))
      (UserInterface|Viewport|AddtoViewport _returnvalue_2 0)
      (Variables|/Script/Engine.PlayerController|SetbShowMouseCursor _returnvalue true)
      (Input|SetInputModeGameandUI _returnvalue _returnvalue_2 "LockAlways" true)
      (Variables|Default|SetEscapeMenu true)
      (else
        (Widget|RemovefromParent _returnvalue_2)
        (Variables|/Script/Engine.PlayerController|SetbShowMouseCursor _returnvalue false)
        (Input|SetInputModeGameOnly _returnvalue)
        (Variables|Default|SetEscapeMenu false)))))

(event Input|KeyboardEvents|O
  (params (Key :type Key%20Structure :default "None")))

(event Input|KeyboardEvents|G
  (params (Key :type Key%20Structure :default "None")))

(event Input|KeyboardEvents|H
  (params (Key :type Key%20Structure :default "None")))

(event Input|KeyboardEvents|Escape
  (params (Key :type Key%20Structure :default "None")))

(event Input|KeyboardEvents|C
  (params (Key :type Key%20Structure :default "None"))
  (:Pressed
    (if (not (Variables|Default|GetisCraftingOpened))
      (bind _outactors (Actor|GetAllActorsOfClass "/Script/Caves_Taint.PlacedItem"))
      (for _array_element _outactors
        (Rendering|SetActorHiddenInGame _array_element true))
      (CallFunction|OpenCrafting)
      (else
        (CallFunction|CloseGuis)
        (UserInterface|Viewport|AddtoViewport (Variables|Default|GetToolBar) 0)
        (Rendering|SetVisibility (Variables|Character|GetMesh) true true)
        (CallFunction|MakeComponentsTree (Variables|/Game/Components/crafting/craftingProcess.craftingProcess_C|Getmesh (Variables|Default|GetcraftingProcess)))
        (Actor|DestroyActor (Variables|Default|GetcraftingProcess))))))

(fn ConstructionScript)

(fn SetEquipmentSave
  (params (Save%20Instance :type Save%20Player%20Object%20Reference))
  (bind _itemsinequipment (Variables|/Game/SaveStructs/savePlayer.savePlayer_C|GetitemsInEquipment Save%20Instance))
  (for _array_element (Variables|Default|GetitemsInEquipment)
    (if (Variables|/Script/Caves_Taint.Item|Getstackable _array_element)
      (Utilities|Array|Add _itemsinequipment (Utilities|Struct|MakeItem (Variables|/Script/Caves_Taint.Item|GetitemName _array_element) (Variables|/Script/Caves_Taint.Item|GetplacedItemClass _array_element) (Variables|/Script/Caves_Taint.Item|Getstackable _array_element) (Variables|/Script/Caves_Taint.Item|Getstack _array_element)))
      (else
        (Utilities|Array|Add _itemsinequipment (Utilities|Struct|MakeItem (Variables|/Script/Caves_Taint.Item|GetitemName _array_element) (Variables|/Script/Caves_Taint.Item|GetplacedItemClass _array_element) (Variables|/Script/Caves_Taint.Item|Getstackable _array_element) 0))))))

(fn LoadEquipmentSaveStruct
  (params (NewParam :type Save%20Player%20Object%20Reference))
  (bind _self self)
  (bind _itemsinequipment (Variables|Default|GetitemsInEquipment))
  (Utilities|Array|Clear (Variables|Default|GetitemsInEquipment))
  (for (_array_element _array_index) (Variables|/Game/SaveStructs/savePlayer.savePlayer_C|GetitemsInEquipment NewParam)
    (if (.stackable _array_element)
      (bind _returnvalue (Game|ConstructObjectfromClass "/Script/Caves_Taint.Item" _self))
      (Variables|/Script/Caves_Taint.Item|SetitemName _returnvalue (.itemname _array_element))
      (Variables|/Script/Caves_Taint.Item|SetplacedItemClass _returnvalue (.placeditemclass _array_element))
      (Variables|/Script/Caves_Taint.Item|Setstackable _returnvalue true)
      (Variables|/Script/Caves_Taint.Item|Setstack _returnvalue (.stack _array_element))
      (Variables|/Script/Caves_Taint.Item|SetequipmentIndex _returnvalue 0)
      (Utilities|Array|Add _itemsinequipment _returnvalue)
      (else
        (bind _returnvalue_2 (Game|ConstructObjectfromClass "/Script/Caves_Taint.Item" _self))
        (Variables|/Script/Caves_Taint.Item|SetitemName _returnvalue_2 (.itemname _array_element))
        (Variables|/Script/Caves_Taint.Item|SetplacedItemClass _returnvalue_2 (.placeditemclass _array_element))
        (Variables|/Script/Caves_Taint.Item|Setstackable _returnvalue_2 false)
        (Variables|/Script/Caves_Taint.Item|SetequipmentIndex _returnvalue_2 _array_index)
        (Utilities|Array|Add _itemsinequipment _returnvalue_2))))
  (Class|PlayerCharacter|UpdateItemIndexes))

(fn OnWorldLoaded
  (params (NewParam :type World%20Object%20Reference)))

(fn SaveWorld
  (bind _outsave (Class|VoxelDataTools|GetCompressedSave (Variables|Default|GetworldReference)))
  (bind _returnvalue (SaveGame|CreateSaveGameObject "/Game/SaveStructs/saveWorld.saveWorld_C"))
  (Variables|/Game/SaveStructs/saveWorld.saveWorld_C|SetworldStruct _returnvalue _outsave)
  (SaveGame|SaveGametoSlot _returnvalue (Utilities|String|Append (Variables|Default|GetcurrentWorldName) "/world")))

(fn LoadWorld)

(fn LoadPlayerParams
  (params (savePlayer :type Save%20Player%20Object%20Reference))
  (bind _playerposition (Variables|/Game/SaveStructs/savePlayer.savePlayer_C|GetplayerPosition savePlayer))
  (Game|SpawnActorfromClass "/Game/SaveStructs/spawnPlatform.spawnPlatform_C" (Math|Transform|MakeTransform (Math|Vector|MakeVector (.x _playerposition) (.y _playerposition) (- (.z _playerposition) 5e+01)) "0, 0, 0" "1,1,1") "Undefined" 0 0)
  (Transformation|SetActorLocation (Math|Vector|MakeVector (.x _playerposition) (.y _playerposition) (.z _playerposition)) false false)
  (Transformation|SetActorRotation (Variables|/Game/SaveStructs/savePlayer.savePlayer_C|GetplayerRotation savePlayer)))

(fn LoadPlayer
  (bind _returnvalue (SaveGame|LoadGamefromSlot (Utilities|String|Append (Variables|Default|GetcurrentWorldName) "/player")))
  (bind _assave_player (Utilities|Casting|CastTosavePlayer _returnvalue))
  (CallFunction|LoadPlayerParams _assave_player)
  (CallFunction|LoadEquipmentSaveStruct _assave_player)
  (Class|PlayerCharacter|ChangeItemMeshinHand))

(fn SetPlayerParamsSave
  (params (save%20instance :type Save%20Player%20Object%20Reference))
  (Variables|/Game/SaveStructs/savePlayer.savePlayer_C|SetplayerPosition save%20instance (Transformation|GetActorLocation))
  (Variables|/Game/SaveStructs/savePlayer.savePlayer_C|SetplayerRotation save%20instance (Transformation|GetActorRotation)))

(fn SavePlayer
  (bind _returnvalue (SaveGame|CreateSaveGameObject "/Game/SaveStructs/savePlayer.savePlayer_C"))
  (CallFunction|SetEquipmentSave _returnvalue)
  (CallFunction|SetPlayerParamsSave _returnvalue)
  (SaveGame|SaveGametoSlot _returnvalue (Utilities|String|Append (Variables|Default|GetcurrentWorldName) "/player")))

(fn SavePlacedItems
  (bind _returnvalue (SaveGame|CreateSaveGameObject "/Game/SaveStructs/chunk.chunk_C"))
  (bind _outactors (Actor|GetAllActorsOfClass "/Script/Caves_Taint.PlacedItem"))
  (for _array_element _outactors
    (bind _asplaced_item (Utilities|Casting|CastToPlacedItemClass (Utilities|GetClass _array_element)))
    (Utilities|Array|Add (Variables|/Game/SaveStructs/chunk.chunk_C|GetplacedItems _returnvalue) (Utilities|Struct|MakeplacedItem _asplaced_item (Transformation|GetActorLocation _array_element)))
    (bind _asitem_holder (Utilities|Casting|CastToItemHolder _array_element))
    (bind _returnvalue_2 (Class|ItemHolder|GetItems _asitem_holder))
    (for _array_element_2 _returnvalue_2
      (bind _newparam1 (CallFunction|CastItemtoItemStruct _array_element_2))
      (Utilities|Array|Add (.savetems (LocalVariables|GettempItemArray)) _newparam1))
    (Utilities|Array|Add (Variables|/Game/SaveStructs/chunk.chunk_C|GetstoredItems _returnvalue) (LocalVariables|GettempItemArray))
    (Utilities|Array|Clear (.savetems (LocalVariables|GettempItemArray))))
  (SaveGame|SaveGametoSlot _returnvalue (Utilities|String|Append (Variables|Default|GetcurrentWorldName) "/chunk")))

(fn CastItemtoItemStruct
  (params (NewParam :type Item%20Object%20Reference%20%28by%20ref%29))
  (if (Variables|/Script/Caves_Taint.Item|Getstackable NewParam)
    (if (Variables|/Script/Caves_Taint.Item|Getstackable NewParam)
      (return (Utilities|Struct|MakeItem (Variables|/Script/Caves_Taint.Item|GetitemName NewParam) (Variables|/Script/Caves_Taint.Item|GetplacedItemClass NewParam) true (Variables|/Script/Caves_Taint.Item|Getstack NewParam))))
    (else
      (return (Utilities|Struct|MakeItem (Variables|/Script/Caves_Taint.Item|GetitemName NewParam) (Variables|/Script/Caves_Taint.Item|GetplacedItemClass NewParam) false 0)))))

(fn CastItemStructtoItem
  (params (itemStruct :type Item%20Structure%20%28by%20ref%29) (Outer :type Object%20Object%20Reference))
  (if (.stackable itemStruct)
    (bind _returnvalue (Game|ConstructObjectfromClass "/Script/Caves_Taint.Item" Outer))
    (Variables|/Script/Caves_Taint.Item|Setstack _returnvalue (.stack itemStruct))
    (Variables|/Script/Caves_Taint.Item|SetitemName _returnvalue (.itemname itemStruct))
    (Variables|/Script/Caves_Taint.Item|SetplacedItemClass _returnvalue (.placeditemclass itemStruct))
    (Variables|/Script/Caves_Taint.Item|Setstackable _returnvalue true)
    (return _returnvalue)
    (else
      (bind _returnvalue_2 (Game|ConstructObjectfromClass "/Script/Caves_Taint.Item" Outer))
      (Variables|/Script/Caves_Taint.Item|SetitemName _returnvalue_2 (.itemname itemStruct))
      (Variables|/Script/Caves_Taint.Item|SetplacedItemClass _returnvalue_2 (.placeditemclass itemStruct))
      (Variables|/Script/Caves_Taint.Item|Setstackable _returnvalue_2 false)
      (return _returnvalue_2))))

(fn SpawnBoxat
  (params (location :type Vector))
  (Game|SpawnActorfromClass "/Script/Caves_Taint.chunkBox" (Math|Transform|MakeTransform (+ (* location 4096) 2048) "0, 0, 0" "1,1,1") "Undefined" 0 0))

(fn CloseGuis
  (bind _returnvalue (Game|GetPlayerController 0))
  (bind _currentlyopenuis (Variables|Default|GetcurrentlyOpenUIs))
  (for _array_element _currentlyopenuis
    (Class|UIBase|OnClose _array_element)
    (Widget|RemovefromParent _array_element))
  (Utilities|Array|Clear _currentlyopenuis)
  (Widget|RemovefromParent (Variables|Default|GetItemStatsShow))
  (Variables|/Script/Engine.PlayerController|SetbShowMouseCursor _returnvalue false)
  (Variables|Default|SetisGuiOpen false)
  (Input|SetInputModeGameOnly _returnvalue)
  (Variables|Default|SetisItemDraggableGuiOpen false)
  (Utilities|FlowControl|Sequence
    (:then_0
      (Rendering|SetActorHiddenInGame (Variables|Default|GetworldReference) false)
      (if (Variables|Default|GetisCraftingOpened)
        (Variables|Default|SetisCraftingOpened false)
        (bind _outactors (Actor|GetAllActorsOfClass "/Script/Caves_Taint.PlacedItem"))
        (for _array_element_2 _outactors
          (Rendering|SetActorHiddenInGame _array_element_2 false))))))

(fn OpenCrafting
  (bind _returnvalue (Game|GetPlayerController 0))
  (bind _characterview (Variables|Default|GetcharacterView))
  (bind _returnvalue_2 (Math|Vector|GetForwardVector _characterview))
  (Rendering|SetVisibility (Variables|Character|GetMesh) false true)
  (Rendering|SetActorHiddenInGame (Variables|Default|GetworldReference) true)
  (Widget|RemovefromParent (Variables|Default|GetToolBar))
  (bind _returnvalue_3 (UserInterface|CreateWidget "/Game/Components/UI/Crafting.Crafting_C" _returnvalue))
  (bind _returnvalue_4 (Game|SpawnActorfromClass "/Game/Components/crafting/craftingProcess.craftingProcess_C" (Math|Transform|MakeTransform (+ (Transformation|GetActorLocation (Game|GetPlayerCharacter 0)) (Math|Vector|MakeVector (* (.x _returnvalue_2) 2.5e+02) (* (.y _returnvalue_2) 2.5e+02) (* (.z _returnvalue_2) 2.5e+02))) "0, 0, 0" "1,1,1") "Undefined" 0 0))
  (Collision|SetCollisionEnabled (Variables|/Game/Components/crafting/craftingProcess.craftingProcess_C|Getmesh _returnvalue_4) "QueryOnly")
  (Variables|Default|SetcraftingProcess _returnvalue_4)
  (UserInterface|Viewport|AddtoViewport _returnvalue_3 0)
  (Utilities|Array|Add (Variables|Default|GetcurrentlyOpenUIs) _returnvalue_3)
  (bind _returnvalue_5 (UserInterface|CreateWidget "/Game/Components/UI/Equipment_BP.Equipment_BP_C" _returnvalue))
  (bind _output_get (Variables|Default|Setequipment _returnvalue_5))
  (Class|Equipment|SetDisplaySize _output_get 2)
  (UserInterface|Viewport|AddtoViewport _output_get 0)
  (Utilities|Array|Add (Variables|Default|GetcurrentlyOpenUIs) _output_get)
  (Variables|Default|SetisCraftingOpened true)
  (Variables|/Script/Engine.PlayerController|SetbShowMouseCursor _returnvalue true)
  (Variables|Default|SetisGuiOpen true)
  (Input|SetInputModeGameandUI _returnvalue (Variables|Default|Getequipment) "LockAlways" true))

(fn EmptyProcess
  (bind _dragitem (Variables|Default|GetdragItem))
  (bind _craftingprocess (Variables|Default|GetcraftingProcess))
  (bind _mesh (Variables|/Game/Components/crafting/craftingProcess.craftingProcess_C|Getmesh _craftingprocess))
  (if (<= (Variables|Default|GetselectedItem) (Utilities|Array|Length (Variables|Default|GetitemsInEquipment)))
    (Components|StaticMesh|SetStaticMesh _mesh (Variables|/Script/Caves_Taint.Item|GetinHandMesh _dragitem))
    (Variables|/Game/Components/crafting/craftingComponent.craftingComponent_C|SetitemName _mesh (Utilities|String|ToString(Name) (Variables|/Script/Caves_Taint.Item|GetitemName _dragitem)))
    (Default|SetLinks _mesh)))

(fn GetMeshinAHand
  (bind _itemsinequipment (Variables|Default|GetitemsInEquipment))
  (if (<= (Variables|Default|GetselectedItem) (Utilities|Array|Length _itemsinequipment))
    (return (Variables|/Script/Caves_Taint.Item|GetinHandMesh (Utilities|Array|Get(acopy) _itemsinequipment (Variables|Default|GetselectedItem))))
    (else
      (return 0))))

(fn MakeComponentsTree
  (params (NewParam :type Crafting%20Component%20Object%20Reference))
  (if (!= NewParam 0)
    (if (> (Utilities|Array|Length (Components|GetChildrenComponents NewParam false)) 0)
      (bind _jsontreeoutput (CallFunction|CreateCraftingBranch (Variables|/Game/Components/crafting/craftingComponent.craftingComponent_C|Getchildrens NewParam)))
      (Development|PrintString (Utilities|String|Replace (Utilities|String|Replace (Utilities|String|Replace (Class|BlueprintJsonLibrary|ToString(JsonObject) (Class|BlueprintJsonLibrary|JsonMakeField (Class|BlueprintJsonLibrary|JsonMake) (Variables|/Game/Components/crafting/craftingComponent.craftingComponent_C|GetitemName NewParam) (Class|BlueprintJsonLibrary|JsonMakeObject _jsontreeoutput))) "\"") ":") ","))
      (if (Utilities|Enum|Equal(Enum) (Utilities|String|Replace (Utilities|String|Replace (Utilities|String|Replace (Class|BlueprintJsonLibrary|ToString(JsonObject) (Class|BlueprintJsonLibrary|JsonMakeField (Class|BlueprintJsonLibrary|JsonMake) (Variables|/Game/Components/crafting/craftingComponent.craftingComponent_C|GetitemName NewParam) (Class|BlueprintJsonLibrary|JsonMakeObject _jsontreeoutput))) "\"") ":") ",") "{Shattered Stone{Shattered Stone3}}")
        (Class|PlayerCharacter|AddItemtoEquipment "testItemmmmmmmmmm" 0 true false 1)))))

(fn AddChildCraftingItem
  (bind _returnvalue (Game|GetPlayerController 0))
  (bind _dragitem (Variables|Default|GetdragItem))
  (bind _hitresult (Game|Player|GetHitResultUnderCursorbyChannel _returnvalue "TraceTypeQuery1" true))
  (bind _inhandmesh (Variables|/Script/Caves_Taint.Item|GetinHandMesh _dragitem))
  (bind (_bblockinghit _binitialoverlap _time _distance _location _impactpoint _normal _impactnormal _physmat _hitactor _hitcomponent) (Collision|BreakHitResult _hitresult))
  (bind _ascrafting_component (Utilities|Casting|CastTocraftingComponent _hitcomponent))
  ;[1 1 1] checks if there are any valid sockets
  (bind _newparam (CallFunction|SetCraftingSockets _ascrafting_component _location))
  (if (Utilities|Name|NotEqual(Name) _newparam "None")
    (bind _ascrafting_process (Utilities|Casting|CastTocraftingProcess _hitactor))
    (bind _returnvalue_2 (AddComponent|AddCraftingComponent _ascrafting_process true))
    (if (!= _inhandmesh 0)
      (Components|StaticMesh|SetStaticMesh _returnvalue_2 _inhandmesh)
      (Default|SetLinks _returnvalue_2)
      (Utilities|Map|Add (Variables|/Game/Components/crafting/craftingComponent.craftingComponent_C|Getchildrens _ascrafting_component) (Math|Conversions|ToInteger(Byte) (Utilities|String|Replace (Utilities|String|ToString(Name) _newparam) "Link_")) _returnvalue_2)
      (Variables|/Game/Components/crafting/craftingComponent.craftingComponent_C|SetitemName _returnvalue_2 (Utilities|String|ToString(Name) (Variables|/Script/Caves_Taint.Item|GetitemName _dragitem)))
      (Variables|/Game/Components/crafting/craftingComponent.craftingComponent_C|SetselfSlotIndex _returnvalue_2 (Math|Conversions|ToInteger(Byte) (Utilities|String|Replace (Utilities|String|ToString(Name) _newparam) "Link_")))
      (Transformation|AttachComponentToComponent _returnvalue_2 _hitcomponent _newparam "KeepRelative" "KeepRelative" "KeepRelative" true))))

(fn CreateCraftingBranch
  (params (NewParam :type Map%20of%20Integers%20to%20Objects))
  (LocalVariables|SettempJson (Class|BlueprintJsonLibrary|JsonMake))
  (bind _values (CallFunction|MapValueBasedonIndex NewParam))
  (for _array_element _values
    (if (> (Utilities|Map|Length (Variables|/Game/Components/crafting/craftingComponent.craftingComponent_C|Getchildrens _array_element)) 0)
      (bind _jsontreeoutput (CallFunction|CreateCraftingBranch (Variables|/Game/Components/crafting/craftingComponent.craftingComponent_C|Getchildrens _array_element)))
      (CallFunction|MakeFildatRuntime (LocalVariables|GettempJson) (Utilities|String|Append (Variables|/Game/Components/crafting/craftingComponent.craftingComponent_C|GetitemName _array_element) (Utilities|String|ToString(Integer) (Variables|/Game/Components/crafting/craftingComponent.craftingComponent_C|GetselfSlotIndex _array_element))) (Class|BlueprintJsonLibrary|JsonMakeObject _jsontreeoutput))
      (else
        (CallFunction|MakeFildatRuntime (LocalVariables|GettempJson) (Utilities|String|Append (Variables|/Game/Components/crafting/craftingComponent.craftingComponent_C|GetitemName _array_element) (Utilities|String|ToString(Integer) (Variables|/Game/Components/crafting/craftingComponent.craftingComponent_C|GetselfSlotIndex _array_element))) (Class|BlueprintJsonLibrary|JsonMakeString)))))
  (return (LocalVariables|GettempJson)))

(fn MakeFildatRuntime
  (params (Object :type Blueprint%20Json%20Object%20Structure%20%28by%20ref%29) (Name :type String) (Value :type Blueprint%20Json%20Value%20Structure%20%28by%20ref%29))
  (return (Class|BlueprintJsonLibrary|JsonMakeField Object Name Value)))

(fn SetCraftingSockets
  (params (component :type Crafting%20Component%20Object%20Reference%20%28by%20ref%29) (location :type Vector))
  (bind _lockedsockets (Variables|/Game/Components/crafting/craftingComponent.craftingComponent_C|GetlockedSockets component))
  (for (_array_element _array_index) (Transformation|GetAllSocketNames component)
    (if (Utilities|Name|Equal(Name) (Utilities|Array|Get(acopy) _lockedsockets _array_index) "None")
      (if (< (Math|Vector|Distance(Vector) (Transformation|GetSocketLocation component _array_element) location) (LocalVariables|GetclosestDistance))
        (LocalVariables|Setindex _array_index)
        (LocalVariables|SetclosestDistance (Math|Vector|Distance(Vector) (Transformation|GetSocketLocation component _array_element) location))
        (LocalVariables|SetclosestSocket _array_element))))
  (Utilities|Array|SetArrayElem _lockedsockets (LocalVariables|Getindex) (Utilities|String|StringToName (Utilities|String|Append (Variables|/Game/Components/crafting/craftingComponent.craftingComponent_C|GetitemName component) (Utilities|String|Replace (Utilities|String|ToString(Name) (LocalVariables|GetclosestSocket)) "Link_"))))
  (return (LocalVariables|GetclosestSocket)))

(fn MakeCraftingBranch
  (params (NewParam :type Crafting%20Component%20Object%20Reference))
  (return ""))

(fn MapValueBasedonIndex
  (params (map :type Map%20of%20Integers%20to%20Objects))
  (bind _values (Utilities|Map|Values map))
  (for _array_element _values
    (Utilities|Array|SetArrayElem (LocalVariables|GettempValues) (Variables|/Game/Components/crafting/craftingComponent.craftingComponent_C|GetselfSlotIndex _array_element) _array_element true))
  (for (_array_element_2 _array_index) (LocalVariables|GettempValues)
    (if (== _array_element_2 0)
      (Utilities|Array|Add (LocalVariables|GetvaluesToRemove) _array_index)))
  (for _array_element_3 (LocalVariables|GetvaluesToRemove)
    (Utilities|Array|RemoveItem (LocalVariables|GettempValues) 0))
  (return (LocalVariables|GettempValues)))

(fn RemoveItemfromCraftingProcess
  (bind _ascrafting_component (Utilities|Casting|CastTocraftingComponent (.HitComponent (Collision|BreakHitResult (.HitResult (Game|Player|GetHitResultUnderCursorbyChannel (Game|GetPlayerController 0) "TraceTypeQuery1" true))))))
  (bind _ascrafting_component_2 (Utilities|Casting|CastTocraftingComponent (Transformation|GetAttachParent _ascrafting_component)))
  (Utilities|Map|Remove (Variables|/Game/Components/crafting/craftingComponent.craftingComponent_C|Getchildrens _ascrafting_component_2) (Variables|/Game/Components/crafting/craftingComponent.craftingComponent_C|GetselfSlotIndex _ascrafting_component))
  (Utilities|Array|SetArrayElem (Variables|/Game/Components/crafting/craftingComponent.craftingComponent_C|GetlockedSockets _ascrafting_component_2) (Variables|/Game/Components/crafting/craftingComponent.craftingComponent_C|GetselfSlotIndex _ascrafting_component) "None")
  (Components|StaticMesh|SetStaticMesh _ascrafting_component 0)
  (Components|DestroyComponent _ascrafting_component))